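; Player controller for a game jam vehicle game that networks tile placement between a host and a connecting client.
; It spawns a TCPListenerGameJam actor on BeginPlay and wraps its hosting, connecting and connection-check calls, acting only on the local controller.
; Sending requires the ready flag set on connecting, and takes the piece shape from VehicleGameMode's selection rather than its own parameter.
; HasNewPosition relays received tile positions and piece types from the listener.
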(event EventBeginPlay
  (bind _returnvalue (Game|SpawnActorfromClass "/Script/JrEngineerSim2017.TCPListenerGameJam" (Math|Transform|MakeTransform "0, 0, 0") "Undefined" 0 0))
  (Variables|Default|SetTCPListener _returnvalue))

(event EventTick
  (params (DeltaSeconds :type Float%20%28single-precision%29)))

(fn ConstructionScript)

(fn ConnecttoHost
  (params (hostAddr :type String))
  (if (Pawn|IsLocalController)
    (Class|TCPListenerGameJam|ConnecttoHost (Variables|Default|GetTCPListener) hostAddr)
    (Variables|Default|Setm_ReadyToPlay true)))

(fn BeginHosting
  (if (Pawn|IsLocalController)
    (bind _outhostaddr (Class|TCPListenerGameJam|BeginHosting (Variables|Default|GetTCPListener)))
    (Variables|Default|SetHostAddr _outhostaddr)
    (Variables|Default|Setm_isHosting true)))

(fn CheckforConnect
  (if (Pawn|IsLocalController)
    (bind _output_get (Variables|Default|Setm_hasConnect (Variables|/Script/JrEngineerSim2017.TCPListenerGameJam|Getm_hasConnection (Variables|Default|GetTCPListener))))
    (return _output_get)
    (else
      (return false))))

(fn SendPlaceTile
  (params (TilePlacePos :type Vector) (TileEnum :type TilePieceEnum%20Enum))
  (if (Pawn|IsLocalController)
    (if (Variables|Default|Getm_ReadyToPlay)
      (Class|TCPListenerGameJam|SendPlaceTile (Variables|Default|GetTCPListener) TilePlacePos (Math|Conversions|ToInteger(Byte) (Variables|/Game/VehicleBP/Blueprints/VehicleGameMode.VehicleGameMode_C|GetSelectedPieceShape (.AsVehicle%20Game%20Mode (Utilities|Casting|CastToVehicleGameMode (Game|GetGameMode)))))))))

(fn HasNewPosition
  (if (Pawn|IsLocalController)
    (if (Pawn|IsLocalController)
      (bind (_position _hasnewposition _tileenum) (Class|TCPListenerGameJam|HasNewPosition (Variables|Default|GetTCPListener)))
      (return _hasnewposition _position (Utilities|Enum|ByteToEnumTilePieceEnum (Math|Conversions|ToByte(Integer) _tileenum)))
      (else
        (return false "0, 0, 0" "NewEnumerator0")))
    (else
      (return false "0, 0, 0" "NewEnumerator0"))))