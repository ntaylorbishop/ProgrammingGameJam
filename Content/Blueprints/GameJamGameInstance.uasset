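; GameJamGameInstance is the game instance that sets up TCP networking when the game starts.
; On Init it spawns a TCPListenerGameJam actor at the origin and keeps a reference to it.
; On any platform other than Android it tells the listener to begin hosting and stores the returned host address.
; A helper function detects Android by comparing the platform name.
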(event EventInit
  (bind _returnvalue (Game|SpawnActorfromClass "/Script/JrEngineerSim2017.TCPListenerGameJam" (Math|Transform|MakeTransform "0, 0, 0") "Undefined" 0 0))
  (Variables|Default|SetTCPListener _returnvalue)
  (if (not (CallFunction|IsonAndroid))
    (bind _outhostaddr (Class|TCPListenerGameJam|BeginHosting (Variables|Default|GetTCPListener)))
    (Variables|Default|SetHostAddr _outhostaddr)))

(fn IsonAndroid
  (bind _returnvalue (Game|GetPlatformName))
  (return (Utilities|Enum|Equal(Enum) _returnvalue "Android")))