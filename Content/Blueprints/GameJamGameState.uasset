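; Game state for a game jam game that places multi-tile shapes built from TileSquare actors.
; SpawnTileShape, gated by CanPlaceTile or hosting, reads the selected shape's tile positions from a data table.
; PlaceTileShapeIfVacant sphere-overlaps every position for existing tiles before spawning one actor per tile.
; As wired, spawns receive a zero position, and CalcTilePosition's grid-scale and Y-flip math is unconnected.
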(event Custom|SpawnTileSquare
  (params (NewTilePosition :type Vector))
  (Game|SpawnActorfromClass "/Game/VehicleBP/Blueprints/TileSquare.TileSquare_C" (Math|Transform|MakeTransform NewTilePosition "0, 0, 0" (Variables|Default|GetTileActorScale3D)) "Undefined" 0 0))

(event EventBeginPlay)

(event EventTick
  (params (DeltaSeconds :type Float%20%28single-precision%29)))

(fn ConstructionScript)

(fn PlaceTileShapeifVacant
  (params (ShapeTiles :type Array%20of%20Vectors) (ShapeOrigin :type Vector))
  (for _array_element ShapeTiles ; beng: First check if vacant.
    (bind _returnvalue (Collision|SphereOverlapActors (Utilities|CalcTilePosition _array_element ShapeOrigin) 1.0 (Utilities|Array|MakeArray "ObjectTypeQuery2") "/Game/VehicleBP/Blueprints/TileSquare.TileSquare_C"))
    (if _returnvalue
      (return false)))
  (for _array_element_2 ShapeTiles ; beng: Then make new one.
    (CallFunction|SpawnTileSquare "0, 0, 0"))
  (return true))

(fn SpawnTileShape
  (params (ShapeOrigin :type Vector))
  (if (or (Variables|Default|GetCanPlaceTile) (Variables|/Game/Blueprints/GameJamGameInstance.GameJamGameInstance_C|Getm_isHosting (.AsGame%20Jam%20Game%20Instance (Utilities|Casting|CastToGameJamGameInstance (Game|GetGameInstance)))))
    (bind _outrownames (DataTable|GetDataTableRowNames "/Game/VehicleBP/Blueprints/TilePiece_DataTable.TilePiece_DataTable"))
    (bind _returnvalue (Utilities|GetDataTableRow "/Game/VehicleBP/Blueprints/TilePiece_DataTable.TilePiece_DataTable" (Utilities|Array|Get(acopy) _outrownames (Math|Conversions|ToInteger(Byte) (Variables|Default|GetSelectedPieceShape))))
      (:then
        (bind _success (CallFunction|PlaceTileShapeifVacant (.TilePositions (Utilities|Struct|BreakTilePiece_DataTableRow _returnvalue)) ShapeOrigin))
        (return _success)))))